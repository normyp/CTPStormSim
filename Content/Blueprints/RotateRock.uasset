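; RotateRock is an actor, by name a rock, that displays a configurable static mesh and spins it through a RotatingMovement component.
; The construction script applies the mesh, rotation rate, pivot translation and local-space flag from Blueprint variables.
; It also creates a dynamic instance of a snow material on the first slot and stores it in AmountOfSnow, without setting any parameters.
; The event graph holds only disabled stub events.
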(event `self.ReceiveBeginPlay`)

(event `self.ReceiveActorBeginOverlap`
  (params (OtherActor :type "Actor Object Reference")))

(event `self.ReceiveTick`
  (params (DeltaSeconds :type "Float (single-precision)")))

(event `Key|W`
  (params (Key :type "Key Structure" :default "AnyKey")))

(fn `UserConstructionScript`
  (bind _rotatingmovement (`self.RotatingMovement`))
  (`StaticMeshComponent.SetStaticMesh` (`self.StaticMesh`) (`self.Mesh`))
  (set `RotatingMovementComponent.RotationRate` (`self.RotationRate`) _rotatingmovement)
  (set `RotatingMovementComponent.PivotTranslation` (`self.Pivot Translation`) _rotatingmovement)
  (set `RotatingMovementComponent.bRotationInLocalSpace` (`self.RotationInLocalSpace`) _rotatingmovement)
  (bind _returnvalue (`PrimitiveComponent.CreateDynamicMaterialInstance` (`self.StaticMesh`) 0 "/Game/Snow_M2_Inst2.Snow_M2_Inst2"))
  (set `self.AmountOfSnow` _returnvalue))